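; Blue coin pickup that spins via a timeline and rewards the third-person character when its capsule enters the sphere.
; Collection advances the character's total and blue coin progress in tenths, adds points, calls ObjectiveComplete and sets BlueCoinComplete from a threshold check.
; The coin then hides its mesh, plays sound and particles, and disables sphere collision rather than destroying itself.
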(event `self.ReceiveBeginPlay`
  ; Rotate coin
  (bind (_direction _newtrack_0) (`Timeline|Timeline` :!via `PlayFromStart`)
    (:`Update`
      (`SceneComponent.K2_SetRelativeRotation` (`self.Cylinder`) (`KismetMathLibrary.MakeRotator` 0.0 0.0 _newtrack_0) false false))))

(event `self.Sphere.OnComponentBeginOverlap`
  (params (OverlappedComponent :type "PrimitiveComponent Object Reference") (OtherActor :type "Actor Object Reference") (OtherComp :type "PrimitiveComponent Object Reference") (OtherBodyIndex :type Integer) (bFromSweep :type Boolean) (SweepResult :type "HitResult Structure (by ref)"))
  ; player over lap coin mechanic
  (bind _asbp_third_person_character (cast `/Game/ThirdPerson/Blueprints/BP_ThirdPersonCharacter` OtherActor))
  (if (== (`Character.CapsuleComponent` _asbp_third_person_character) OtherComp)
    (set `/Game/ThirdPerson/Blueprints/BP_ThirdPersonCharacter.totalCoin` (+ (`/Game/ThirdPerson/Blueprints/BP_ThirdPersonCharacter.totalCoin` _asbp_third_person_character) 0.1) _asbp_third_person_character)
    (`/Game/ThirdPerson/Blueprints/BP_ThirdPersonCharacter.Objective_Complete` _asbp_third_person_character)
    (`SceneComponent.SetVisibility` (`self.Cylinder`) false false)
    (set `/Game/ThirdPerson/Blueprints/BP_ThirdPersonCharacter.BlueCoin` (+ (`/Game/ThirdPerson/Blueprints/BP_ThirdPersonCharacter.BlueCoin` _asbp_third_person_character) 0.1) _asbp_third_person_character)
    (set `/Game/ThirdPerson/Blueprints/BP_ThirdPersonCharacter.PlayerPoints` (+ (`/Game/ThirdPerson/Blueprints/BP_ThirdPersonCharacter.PlayerPoints` _asbp_third_person_character) 300.0) _asbp_third_person_character)
    (`GameplayStatics.PlaySound2D` "/Game/Sound/coin-pickup-98269.coin-pickup-98269" 1.0 1.0 0.0 null null)
    (set `/Game/ThirdPerson/Blueprints/BP_ThirdPersonCharacter.blueCoinComplete` (> (`/Game/ThirdPerson/Blueprints/BP_ThirdPersonCharacter.BlueCoin` _asbp_third_person_character) 0.9) _asbp_third_person_character)
    (`ActorComponent.Activate` (`self.ParticleSystem`) false)
    (`PrimitiveComponent.SetCollisionEnabled` (`self.Sphere`) "NoCollision")))

(fn `UserConstructionScript`)