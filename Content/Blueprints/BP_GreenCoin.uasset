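; BP_GreenCoin is a pickup coin that raises the player's HP.
; When the third-person character's capsule overlaps its Sphere, it adds IncreaseHP to PlayerHP with no clamp in this graph.
; It then hides the Cylinder mesh, disables Sphere collision, activates a Niagara effect and plays a 2D pickup sound.
; The actor is never destroyed, so disabling collision is what prevents a second pickup.
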(event `self.Sphere.OnComponentBeginOverlap`
  (params (OverlappedComponent :type "PrimitiveComponent Object Reference") (OtherActor :type "Actor Object Reference") (OtherComp :type "PrimitiveComponent Object Reference") (OtherBodyIndex :type Integer) (bFromSweep :type Boolean) (SweepResult :type "HitResult Structure (by ref)"))
  ; player over lap coin mechanic to increase HP
  (bind _asbp_third_person_character (cast `/Game/ThirdPerson/Blueprints/BP_ThirdPersonCharacter` OtherActor))
  (if (== (`Character.CapsuleComponent` _asbp_third_person_character) OtherComp)
    (set `/Game/ThirdPerson/Blueprints/BP_ThirdPersonCharacter.PlayerHP` (+ (`/Game/ThirdPerson/Blueprints/BP_ThirdPersonCharacter.PlayerHP` _asbp_third_person_character) (`self.IncreaseHP`)) _asbp_third_person_character)
    (`SceneComponent.SetVisibility` (`self.Cylinder`) false false)
    (`PrimitiveComponent.SetCollisionEnabled` (`self.Sphere`) "NoCollision")
    (`ActorComponent.Activate` (`self.Niagara`) false)
    (`GameplayStatics.PlaySound2D` "/Game/Sound/Audio/item-pick-up-38258.item-pick-up-38258" 1.0 1.0 0.0 null null)))

(fn `UserConstructionScript`)