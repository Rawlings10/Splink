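; BP_OrangeCoin is a pickup coin that applies damage to the player character on contact.
; When the Sphere begins overlapping a BP_ThirdPersonCharacter's capsule, it applies Coindamge to player 0's character rather than the overlapping actor reference.
; It then hides the Cylinder mesh, disables Sphere collision, activates its particle system and plays a 2D sound.
; The actor stays in the level, as it is never destroyed here.
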(event `self.Sphere.OnComponentBeginOverlap`
  (params (OverlappedComponent :type "PrimitiveComponent Object Reference") (OtherActor :type "Actor Object Reference") (OtherComp :type "PrimitiveComponent Object Reference") (OtherBodyIndex :type Integer) (bFromSweep :type Boolean) (SweepResult :type "HitResult Structure (by ref)"))
  (bind _asbp_third_person_character (cast `/Game/ThirdPerson/Blueprints/BP_ThirdPersonCharacter` OtherActor))
  (if (== (`Character.CapsuleComponent` _asbp_third_person_character) OtherComp)
    (`GameplayStatics.ApplyDamage` (`GameplayStatics.GetPlayerCharacter` 0) (`self.coindamge`))
    (`SceneComponent.SetVisibility` (`self.Cylinder`) false false)
    (`PrimitiveComponent.SetCollisionEnabled` (`self.Sphere`) "NoCollision")
    (`ActorComponent.Activate` (`self.ParticleSystem`) false)
    (`GameplayStatics.PlaySound2D` "/Game/Sound/086409_retro-gun-shot-81545.086409_retro-gun-shot-81545" 1.0 1.0 0.0 null null)))

(fn `UserConstructionScript`)